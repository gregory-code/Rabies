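; BP_BoltHead is a player Blueprint, apparently for the Bolt character's head, that sets up animation and shows muzzle flashes.
; On BeginPlay it calls SetOwnerCharacter on the RAnimInstanceBase anim instances of Torso and Flying, stopping if a cast fails.
; CharacterShootParticle forwards to SpawnClientParticle, which attaches the NS_MuzzleFlash Niagara system to Mesh at the shot's start, oriented by its forward value.
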(event Custom|SpawnClientParticle
  (params (startPos :type Vector) (endPos :type Vector) (startForward :type Rotator))
  (Niagara|SpawnSystemAttached "/Game/VFX/NS/NS_MuzzleFlash.NS_MuzzleFlash" (Variables|Character|GetMesh) "" startPos startForward "KeepWorldPosition" false))

(event EventBeginPlay
  (bind _torso (Variables|Default|GetTorso))
  (bind _flying (Variables|Default|GetFlying))
  (bind _asranim_instance_base (Utilities|Casting|CastToRAnimInstanceBase (Components|SkeletalMesh|GetAnimInstance _torso)))
  (Class|RAnimInstanceBase|SetOwnerCharacter _asranim_instance_base _torso)
  (bind _asranim_instance_base_2 (Utilities|Casting|CastToRAnimInstanceBase (Components|SkeletalMesh|GetAnimInstance _flying)))
  (Class|RAnimInstanceBase|SetOwnerCharacter _asranim_instance_base_2 _flying))

(event EventCharacterShootParticle
  (params (startPos :type Vector :default "0, 0, 0") (endPos :type Vector :default "0, 0, 0") (startForward :type Rotator :default "0, 0, 0"))
  (CallFunction|SpawnClientParticle startPos endPos startForward))

(fn ConstructionScript)