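; Player controller for the main menu that sets Game and UI input on BeginPlay and offers a Backspace shortcut for changing level.
; With authority, Backspace calls LoadLevel, which issues a ServerTravel console command aimed at Facility_Courtyard; without authority it only logs a placeholder message.
; The local-only logic that creates the WBP_ConnectMenu widget and shows the cursor is disconnected and never runs.
; LoadLevelOnServer is an empty stub.
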(event Custom|LoadLevel
  (Development|ExecuteConsoleCommand "ServerTravel/Game/Levels/Facility_Courtyard" 0))

(event EventBeginPlay
  (Input|SetInputModeGameandUI self 0 "DoNotLock" true false))

(event EventTick
  (params (DeltaSeconds :type Float%20%28single-precision%29)))

(event Input|KeyboardEvents|Backspace
  (params (Key :type Key%20Structure :default "None"))
  (:Pressed
    (if (Ability|HasAuthority)
      (CallFunction|LoadLevel)
      (else
        (Utilities|String|LogString "Hello")))))

(fn ConstructionScript)

(fn LoadLevelonServer)